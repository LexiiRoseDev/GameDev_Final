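; Main game mode for a creature breeding game, acting as the hub for tool UI, debug hotkeys and pausing.
; BeginPlay enables input on the game mode and creates the widgets, showing debug, designer and spawner UI immediately while breed and trait menus wait for hotkeys.
; Other keys switch game speed, destroy tracked creatures, print species and trait-count info, or drive debug controls.
; Tab toggles pause with a pause menu and matching input mode.
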(event EventBeginPlay
  (bind _returnvalue (Game|GetPlayerController 0))
  (Input|EnableInput _returnvalue)
  (bind _returnvalue_2 (UserInterface|CreateWidget "/Game/Blueprints/Widgets/Temp-Debug/WBP_BreedMenu.WBP_BreedMenu_C" _returnvalue))
  (Variables|Default|SetBreed%20Menu _returnvalue_2)
  (bind _returnvalue_3 (UserInterface|CreateWidget "/Game/Blueprints/Widgets/Temp-Debug/WBP_TraitApplier.WBP_TraitApplier_C" _returnvalue))
  (Variables|Default|SetTrait%20Applier%20Menu _returnvalue_3)
  (bind _returnvalue_4 (UserInterface|CreateWidget "/Game/Blueprints/Widgets/WBP_DebugMenu.WBP_DebugMenu_C" _returnvalue))
  (Variables|Default|SetDebugMenu _returnvalue_4)
  (UserInterface|Viewport|AddtoViewport (Variables|Default|GetDebugMenu) 0)
  (bind _returnvalue_5 (UserInterface|CreateWidget "/Game/Blueprints/Widgets/WBP_DesignerTab.WBP_DesignerTab_C" _returnvalue))
  (UserInterface|Viewport|AddtoViewport _returnvalue_5 0)
  (bind _returnvalue_6 (UserInterface|CreateWidget "/Game/Blueprints/Widgets/WBP_SpawnerToolButton.WBP_SpawnerToolButton_C" _returnvalue))
  (bind _output_get (Variables|Default|SetSpawn%20Species%20Widget _returnvalue_6))
  (UserInterface|Viewport|AddtoViewport _output_get 0))

(event Input|KeyboardEvents|2
  (params (Key :type Key%20Structure :default "None"))
  ;[0.15 0.15 0.15 0.5] Debugs
  (:Pressed
    (Utilities|Time|SetGlobalTimeDilation 2.0)
    (Development|PrintString "Double Speed")))

(event Input|KeyboardEvents|K
  (params (Key :type Key%20Structure :default "None"))
  (bind _creatures (Variables|Default|GetCreatures))
  ;[0.15 0.15 0.15 0.5] Debugs
  (:Pressed
    (for _array_element _creatures
      (Actor|DestroyActor (.Actor (Utilities|Struct|BreakST_Creature _array_element))))
    (Utilities|Array|Clear _creatures)))

(event Input|KeyboardEvents|R
  (params (Key :type Key%20Structure :default "None"))
  ;[0.15 0.15 0.15 0.5] Debugs
  (:Pressed
    (bind _outactors (Actor|GetAllActorsOfClass "/Game/Blueprints/Creatures/BPP_Creature.BPP_Creature_C"))
    (for _array_element _outactors
      (Development|PrintString (Utilities|String|ToString(Integer) (Variables|/Game/Blueprints/Creatures/BPP_Creature.BPP_Creature_C|GetSpeciesID _array_element)))
      (Development|PrintText (Utilities|Text|FormatText "HT: {L}" (Utilities|Array|Length (Variables|/Game/Blueprints/Creatures/BPP_Creature.BPP_Creature_C|GetHeld%20Traits _array_element)))))))

(event Input|KeyboardEvents|E
  (params (Key :type Key%20Structure :default "None"))
  ;[0.15 0.15 0.15 0.5] Debugs
  (:Pressed
    (for _array_element (Variables|Default|GetSpecies)
      (Development|PrintText (.speciesname _array_element)))))

(event Input|KeyboardEvents|T
  (params (Key :type Key%20Structure :default "None"))
  ;[0.15 0.15 0.15 0.5] Breed menu debug
  (:Pressed
    (UserInterface|Viewport|AddtoViewport (Variables|Default|GetTrait%20Applier%20Menu) 0)))

(event Input|KeyboardEvents|1
  (params (Key :type Key%20Structure :default "None"))
  ;[0.15 0.15 0.15 0.5] Debugs
  (:Pressed
    (Utilities|Time|SetGlobalTimeDilation 1.0)
    (Development|PrintString "Normal Speed")))

(event Input|KeyboardEvents|3
  (params (Key :type Key%20Structure :default "None"))
  ;[0.15 0.15 0.15 0.5] Debug Menu
  (:Pressed
    (Default|DebugControls (Variables|Default|GetDebugMenu))))

(event Input|KeyboardEvents|B
  (params (Key :type Key%20Structure :default "None"))
  ;[0.15 0.15 0.15 0.5] Breed menu debug
  (:Pressed
    (UserInterface|Viewport|AddtoViewport (Variables|Default|GetBreed%20Menu) 0)))

(event Input|KeyboardEvents|Tab
  (params (Key :type Key%20Structure :default "None"))
  (bind _returnvalue (Game|GetPlayerController 0))
  ;[0.15 0.15 0.15 0.5] PauseMenu
  (:Pressed
    (if (Game|IsGamePaused)
      (Utilities|FlowControl|Sequence
        (:then_0
          (Widget|RemovefromParent (stale _returnvalue_2)))
        (:then_1
          (Game|SetGamePaused false)
          (Input|SetInputModeGameOnly _returnvalue true)
          (Variables|/Script/Engine.PlayerController|SetbShowMouseCursor _returnvalue true)))
      (else
        (bind _returnvalue_2 (UserInterface|CreateWidget "/Game/Blueprints/Widgets/WBP_PauseMenu.WBP_PauseMenu_C" _returnvalue))
        (UserInterface|Viewport|AddtoViewport _returnvalue_2 100)
        (Game|SetGamePaused true)
        (Input|SetInputModeGameandUI _returnvalue 0 "DoNotLock" false true)
        (Variables|/Script/Engine.PlayerController|SetbShowMouseCursor _returnvalue true)))))

(fn ConstructionScript)