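; Free camera Blueprint with planar movement, orbit around a pivot and mouse cursor control via Enhanced Input.
; Move input sweeps the Sphere along the Pivot's right and forward vectors, scaled by speed.
; Holding the orbit input hides the cursor and switches to game-only input, letting look input yaw the Pivot and pitch the SpringArm.
; The pitch clamp limits each input delta, not the accumulated arm angle.
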(event Input|EnhancedActionEvents|EnhancedInputActionIA_Move
  (params (ActionValue :type Vector%202D%20Structure) (ElapsedSeconds :type Float%20%28double-precision%29) (TriggeredSeconds :type Float%20%28double-precision%29) (InputAction :type Input%20Action%20Object%20Reference :default "/Game/Input/IA_Move.IA_Move"))
  (bind (_x _y) (Math|Vector2D|BreakVector2D ActionValue))
  (bind _pivot (Variables|Default|GetPivot))
  ;[0.15 0.15 0.15 0.5] X is Y. Y is X.
  (Transformation|AddWorldOffset (Variables|Default|GetSphere) (* (+ (* _x (Math|Vector|GetRightVector _pivot)) (* _y (Math|Vector|GetForwardVector _pivot))) (Variables|Default|GetCamMoveSpeed)) true false))

(event Input|EnhancedActionEvents|EnhancedInputActionIA_Orbit
  (params (ActionValue :type Boolean) (ElapsedSeconds :type Float%20%28double-precision%29) (TriggeredSeconds :type Float%20%28double-precision%29) (InputAction :type Input%20Action%20Object%20Reference :default "/Game/Input/IA_Orbit.IA_Orbit"))
  (bind _returnvalue (Game|GetPlayerController 0))
  ;[0.15 0.15 0.15 0.5] Set is orbit to true by holding right click. Will hide mouse cursor and allow you to rotate camera around the object.
  (:Started
    (Variables|Default|SetisOrbit true)
    (Variables|/Script/Engine.PlayerController|SetbShowMouseCursor _returnvalue false)
    (Input|SetInputModeGameOnly _returnvalue false))
  (:Completed
    (Variables|Default|SetisOrbit false)
    (Variables|/Script/Engine.PlayerController|SetbShowMouseCursor _returnvalue true)
    (Input|SetInputModeGameandUI _returnvalue 0 "DoNotLock" true false)))

(event Input|EnhancedActionEvents|EnhancedInputActionIA_Look
  (params (ActionValue :type Vector%202D%20Structure) (ElapsedSeconds :type Float%20%28double-precision%29) (TriggeredSeconds :type Float%20%28double-precision%29) (InputAction :type Input%20Action%20Object%20Reference :default "/Game/Input/IA_Look.IA_Look"))
  ;[0.15 0.15 0.15 0.5] While holding right click, can rotate camera around pivot point.
  (if (Variables|Default|GetisOrbit)
    (Transformation|AddLocalRotation (Variables|Default|GetPivot) (Math|Rotator|MakeRotator 0.0 0.0 (* (.x ActionValue) (Variables|Default|GetCamRotMult))) false false)
    (Transformation|AddLocalRotation (Variables|Default|GetSpringArm) (Math|Rotator|MakeRotator 0.0 (Math|Float|Clamp(Float) (* (.y ActionValue) (Variables|Default|GetCamRotMult)) -8e+01 8e+01) 0.0) false false)))

(event EventBeginPlay
  (bind _returnvalue (Game|GetPlayerController 0))
  ;[0.15 0.15 0.15 0.5] Enables input.
  (Input|AddMappingContext (PlayerController|LocalPlayerSubsystems|GetEnhancedInputLocalPlayerSubsystem _returnvalue) "/Game/Input/IMC_FreeCam.IMC_FreeCam" 0 "(bIgnoreAllPressedKeysUntilRelease=True,bForceImmediately=False,bNotifyUserSettings=False)")
  (Input|SetInputModeGameandUI _returnvalue 0 "DoNotLock" true false)
  (Variables|/Script/Engine.PlayerController|SetbShowMouseCursor _returnvalue true))

(fn ConstructionScript)