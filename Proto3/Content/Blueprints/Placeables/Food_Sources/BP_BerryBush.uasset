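; BP_BerryBush is a placeable berry bush, filed under food sources, that can be removed with the eraser tool.
; On BeginPlay it randomly picks a blueberry, cherry or orange mesh for its static mesh component.
; While the delete tool is active, cursor hover applies a red outline overlay material to all its mesh components and a click destroys the actor.
; Moving the cursor off clears the overlay.
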(event EventBeginPlay
  (bind _bushsm (Variables|Default|GetBushSM))
  (switch int (Math|Random|RandomIntegerinRange 0 2)
    (:0
      (Components|StaticMesh|SetStaticMesh _bushsm "/Game/Assets/SM/SM_BushBlueBerry.SM_BushBlueBerry"))
    (:1
      (Components|StaticMesh|SetStaticMesh _bushsm "/Game/Assets/SM/SM_BushCherry.SM_BushCherry"))
    (:2
      (Components|StaticMesh|SetStaticMesh _bushsm "/Game/Assets/SM/SM_Bushorange.SM_Bushorange"))))

(event MouseInput|EventActorBeginCursorOver
  ;[0.15 0.01891 0.01891 0.5] Enable Deletion with Eraser Tool
  (bind _active_ (CallFunction|DeleteToolActive?))
  (if _active_
    (for _array_element (Actor|GetComponentsByClass "/Script/Engine.MeshComponent")
      (Rendering|Material|SetOverlayMaterial _array_element "/Game/Assets/Materials/M_RedOutline1.M_RedOutline1" :!class /Script/Engine.MeshComponent))))

(event MouseInput|EventActorEndCursorOver
  ;[0.15 0.01891 0.01891 0.5] Enable Deletion with Eraser Tool
  (for _array_element (Actor|GetComponentsByClass "/Script/Engine.MeshComponent")
    (Rendering|Material|SetOverlayMaterial _array_element 0 :!class /Script/Engine.MeshComponent)))

(event EventTick
  (params (DeltaSeconds :type Float%20%28single-precision%29)))

(event MouseInput|EventActorOnClicked
  (params (ButtonPressed :type Key%20Structure :default "None"))
  ;[0.15 0.01891 0.01891 0.5] Enable Deletion with Eraser Tool
  (bind _active_ (CallFunction|DeleteToolActive?))
  (if _active_
    (Actor|DestroyActor)))

(fn ConstructionScript)