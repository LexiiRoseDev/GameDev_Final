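; BP_FenceCorner is a placeable fence corner structure that supports deletion with the eraser tool.
; While the delete tool is active, cursor hover applies a red outline overlay material to every mesh component and a click destroys the actor.
; Ending hover clears the overlay regardless of tool state.
; BeginPlay, Tick, overlap and the construction script contain no logic.
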(event EventBeginPlay)

(event MouseInput|EventActorBeginCursorOver
  ;[0.15 0.01891 0.01891 0.5] Enable Deletion with Eraser Tool
  (bind _active_ (CallFunction|DeleteToolActive?))
  (if _active_
    (for _array_element (Actor|GetComponentsByClass "/Script/Engine.MeshComponent")
      (Rendering|Material|SetOverlayMaterial _array_element "/Game/Assets/Materials/M_RedOutline1.M_RedOutline1" :!class /Script/Engine.MeshComponent))))

(event MouseInput|EventActorEndCursorOver
  ;[0.15 0.01891 0.01891 0.5] Enable Deletion with Eraser Tool
  (for _array_element (Actor|GetComponentsByClass "/Script/Engine.MeshComponent")
    (Rendering|Material|SetOverlayMaterial _array_element 0 :!class /Script/Engine.MeshComponent)))

(event Collision|EventActorBeginOverlap
  (params (OtherActor :type Actor%20Object%20Reference)))

(event MouseInput|EventActorOnClicked
  (params (ButtonPressed :type Key%20Structure :default "None"))
  ;[0.15 0.01891 0.01891 0.5] Enable Deletion with Eraser Tool
  (bind _active_ (CallFunction|DeleteToolActive?))
  (if _active_
    (Actor|DestroyActor)))

(event EventTick
  (params (DeltaSeconds :type Float%20%28single-precision%29)))

(fn ConstructionScript)