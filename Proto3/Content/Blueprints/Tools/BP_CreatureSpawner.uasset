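; Creature spawner that registers itself with GM_MainGameMode and spawns random-sized batches of BPP_Creature scattered around its location.
; NewSpecies, called by a widget, spawns a batch while under the species cap, using a DoOnce to create one species entry per batch.
; SpawnChildren spawns offspring with bred base values and held traits, keeping the given species ID and advancing the generation.
; Both paths initiate each creature and record it in the game mode's creature list.
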(event Custom|New%20Species
  ;[0.15 0.15 0.15 0.5] Called by widget
  (bind _asgm_main_game_mode (Utilities|Casting|CastToGM_MainGameMode (Game|GetGameMode)))
  (if (< (Variables|/Game/Blueprints/GM_MainGameMode.GM_MainGameMode_C|GetLivingSpecies _asgm_main_game_mode) (Variables|/Game/Blueprints/GM_MainGameMode.GM_MainGameMode_C|GetMaxSpecies _asgm_main_game_mode))
    (CallFunction|SpawnCreatures)
    (Math|Integer|IncrementInt (Variables|/Game/Blueprints/GM_MainGameMode.GM_MainGameMode_C|GetLivingSpecies _asgm_main_game_mode))))

(event EventBeginPlay
  ;[0.15 0.15 0.15 0.5] Lets you press space
  (Input|EnableInput (Game|GetPlayerController 0))
  (bind _asgm_main_game_mode (Utilities|Casting|CastToGM_MainGameMode (Game|GetGameMode)))
  (Variables|/Game/Blueprints/GM_MainGameMode.GM_MainGameMode_C|SetCreatureSpawner _asgm_main_game_mode self))

(fn ConstructionScript)

(fn SpawnCreatures
  (bind _defaultsceneroot (Variables|Default|GetDefaultSceneRoot))
  (bind _spawned (LocalVariables|GetSpawned))
  (bind _spawnedcreatures (LocalVariables|GetSpawnedCreatures))
  (bind _returnvalue (Transformation|GetWorldLocation _defaultsceneroot))
  ;[0.15 0.15 0.15 0.5] Only spawn a random quantity between the minimum and maximum
  (bind _output_get (LocalVariables|SetSpawnCount (Math|Random|RandomIntegerinRange (Variables|Default|GetMinSpawnCount) (Variables|Default|GetMaxSpawnCount))))
  (while (< (LocalVariables|GetSpawned) _output_get)
    ;[0.15 0.15 0.15 0.5] Spawn the creature and then check it exists, before incrementing the spawned variable for the while loop. Then add that creatures to the list of spawned creatures for this instance of spawnings.
    (bind _returnvalue_2 (Game|SpawnActorfromClass :Class "/Game/Blueprints/Creatures/BPP_Creature.BPP_Creature_C" :SpawnTransform (Math|Transform|MakeTransform (Math|Vector|MakeVector (+ (.x _returnvalue) (Math|Random|RandomFloatinRange -5e+02 5e+02)) (+ (.y _returnvalue) (Math|Random|RandomFloatinRange -5e+02 5e+02)) (.z _returnvalue)) (Math|Rotator|MakeRotator 0.0 (Math|Random|RandomFloatinRange -1.0 1.0) (Math|Random|RandomFloatinRange 0.0 3.6e+02))) :CollisionHandlingOverride "AlwaysSpawn" :TransformScaleMethod "MultiplyWithRoot" :Instigator 0))
    (Utilities|IsValid _returnvalue_2
      (:Is%20Valid
        (Math|Integer|IncrementInt _spawned
          (:%20%20
            (Utilities|Array|Insert (LocalVariables|GetSpawnedCreatures) _returnvalue_2)
            ;[0.15 0.15 0.15 0.5] Only once per set of creatures spawned, add a species to the gamemode's species list for that set of creatures
            (Utilities|FlowControl|DoOnce false
              (:Completed
                (bind _species (CallFunction|AddtoSpecies _returnvalue_2)))))))
      (:Is%20Not%20Valid
        (Math|Integer|IncrementInt _spawned))))
  ;[0.15 0.15 0.15 0.5] After all creatures in set have spawned, give all of those creatures a species ID based on the new species created, then clear the list of spawned creatures to ready it for the next set, and reset the do-once for creating a new species. Also initiates creature once species ID is allocated and adds them to the gamemode's creature list
  (for _array_element _spawnedcreatures
    (Variables|/Game/Blueprints/Creatures/BPP_Creature.BPP_Creature_C|SetSpeciesID _array_element (.speciesid _species))
    (bind _asgm_main_game_mode (Utilities|Casting|CastToGM_MainGameMode (Game|GetGameMode)))
    (bind _result (Math|Integer|IncrementInt (Variables|/Game/Blueprints/GM_MainGameMode.GM_MainGameMode_C|GetLatestCreatureID _asgm_main_game_mode))
      (:%20%20
        (bind _name (Default|InitiateCreature _array_element))
        (Utilities|Array|Insert (Variables|/Game/Blueprints/GM_MainGameMode.GM_MainGameMode_C|GetCreatures _asgm_main_game_mode) (Utilities|Struct|MakeST_Creature (.speciesid _species) 1 _name _result _array_element)))))
  (Utilities|Array|Clear _spawnedcreatures)
  (Utilities|FlowControl|DoOnce false) ; enters at Reset
)

(fn AddtoSpecies
  (params (Creature :type BPP%20Creature%20Object%20Reference))
  ;[0.15 0.15 0.15 0.5] Creates a new species and adds it to the gamemode's list. Gives it an ID one above the previous
  (bind _asgm_main_game_mode (Utilities|Casting|CastToGM_MainGameMode (Game|GetGameMode)))
  (Utilities|Array|Insert (Variables|/Game/Blueprints/GM_MainGameMode.GM_MainGameMode_C|GetSpecies _asgm_main_game_mode) (Utilities|Struct|MakeST_Species (Utilities|Array|Length (Variables|/Game/Blueprints/GM_MainGameMode.GM_MainGameMode_C|GetSpecies _asgm_main_game_mode)) (Utilities|Text|FormatText "Species {ID}" (+ (Utilities|Array|Length (Variables|/Game/Blueprints/GM_MainGameMode.GM_MainGameMode_C|GetSpecies _asgm_main_game_mode)) 1)) 1 false Creature))
  (return (Utilities|Struct|MakeST_Species (Utilities|Array|Length (Variables|/Game/Blueprints/GM_MainGameMode.GM_MainGameMode_C|GetSpecies _asgm_main_game_mode)) (Utilities|Text|FormatText "Species {ID}" (+ (Utilities|Array|Length (Variables|/Game/Blueprints/GM_MainGameMode.GM_MainGameMode_C|GetSpecies _asgm_main_game_mode)) 1)) 1 false Creature)))

(fn SpawnChildren
  (params (Base%20Vals :type ST%20Creature%20Base%20Values%20Structure) (HT :type Array%20of%20ST%20Held%20Trait%20Structures) (Species%20ID :type Integer) (Previous%20Generation :type Integer))
  (bind _returnvalue (+ Previous%20Generation 1))
  (bind _defaultsceneroot (Variables|Default|GetDefaultSceneRoot))
  (bind _spawnedcreatures (LocalVariables|GetSpawnedCreatures))
  (bind _returnvalue_2 (Transformation|GetWorldLocation _defaultsceneroot))
  ;[0.15 0.15 0.15 0.5] Grab the base values generated during breeding
  (LocalVariables|SetBase%20Values Base%20Vals)
  ;[0.15 0.15 0.15 0.5] Only spawn a random quantity between the minimum and maximum
  (bind _output_get (LocalVariables|SetSpawnCount (Math|Random|RandomIntegerinRange (Variables|Default|GetMinSpawnCount) (Variables|Default|GetMaxSpawnCount))))
  (while (< (LocalVariables|GetSpawned) _output_get)
    ;[0.15 0.15 0.15 0.5] Spawn the creature and then check it exists, before incrementing the spawned variable for the while loop. Then add that creatures to the list of spawned creatures for this instance of spawnings.
    (bind _returnvalue_3 (Game|SpawnActorfromClass "/Game/Blueprints/Creatures/BPP_Creature.BPP_Creature_C" (Math|Transform|MakeTransform (Math|Vector|MakeVector (+ (.x _returnvalue_2) (Math|Random|RandomFloatinRange -5e+02 5e+02)) (+ (.y _returnvalue_2) (Math|Random|RandomFloatinRange -5e+02 5e+02)) (.z _returnvalue_2)) (Math|Rotator|MakeRotator 0.0 (Math|Random|RandomFloatinRange -1.0 1.0) (Math|Random|RandomFloatinRange 0.0 3.6e+02))) "AlwaysSpawn" "MultiplyWithRoot" 0 (LocalVariables|GetBase%20Values) HT 0))
    (Utilities|IsValid _returnvalue_3
      (:Is%20Valid
        (Math|Integer|IncrementInt (LocalVariables|GetSpawned)
          (:%20%20
            (Utilities|Array|Insert (LocalVariables|GetSpawnedCreatures) _returnvalue_3))))))
  ;[0.15 0.15 0.15 0.5] After all creatures in set have spawned, give all of those creatures a species ID based on the new species created, then clear the list of spawned creatures to ready it for the next set, and reset the do-once for creating a new species. Also initiates creature once species ID is allocated and adds them to the gamemode's creature list
  (for _array_element _spawnedcreatures
    (Variables|/Game/Blueprints/Creatures/BPP_Creature.BPP_Creature_C|SetSpeciesID _array_element Species%20ID)
    (Variables|/Game/Blueprints/Creatures/BPP_Creature.BPP_Creature_C|SetGeneration _array_element _returnvalue)
    (bind _asgm_main_game_mode (Utilities|Casting|CastToGM_MainGameMode (Game|GetGameMode)))
    (bind _result (Math|Integer|IncrementInt (Variables|/Game/Blueprints/GM_MainGameMode.GM_MainGameMode_C|GetLatestCreatureID _asgm_main_game_mode))
      (:%20%20
        (bind _name (Default|InitiateCreature _array_element))
        (Utilities|Array|Insert (Variables|/Game/Blueprints/GM_MainGameMode.GM_MainGameMode_C|GetCreatures _asgm_main_game_mode) (Utilities|Struct|MakeST_Creature Species%20ID _returnvalue _name _result _array_element)))))
  (Utilities|Array|Clear _spawnedcreatures))