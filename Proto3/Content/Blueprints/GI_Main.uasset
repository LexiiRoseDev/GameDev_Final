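; Game Instance that saves and restores the creature world and free camera through a BP_SaveGame slot.
; SaveCurrentData builds a fresh save from the level name, every creature's data, the game mode's latest creature ID and camera settings, then requests the disk write.
; LoadGameData reads the slot, flags RestorePending and reopens the saved level.
; LoadSavedData respawns creatures and reapplies camera settings, with no live call in this graph.
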(event EventInit)

(event EventLoadGameData
  ;[0.15 0.15 0.15 0.5] Load Game Data
  (bind _returnvalue (SaveGame|LoadGamefromSlot (Variables|Default|GetSlot%20Name)))
  (bind _asbp_save_game (Utilities|Casting|CastToBP_SaveGame _returnvalue))
  (bind _output_get (Variables|Default|SetSaveData _asbp_save_game))
  (Variables|Default|SetRestorePending true)
  (Game|OpenLevel(byName) (Variables|/Game/Blueprints/Save-Load/BP_SaveGame.BP_SaveGame_C|GetSavedLevel _output_get)))

(event EventSaveGameData
  ;[0.15 0.15 0.15 0.5] Save Game Data
  (bind _returnvalue (SaveGame|SaveGametoSlot (Variables|Default|GetSaveData) (Variables|Default|GetSlot%20Name)))
  (if _returnvalue
    (Development|PrintString "Save Success")
    (else
      (Development|PrintString "Save Failed"))))

(fn SaveCurrentData
  (bind _returnvalue (Game|GetCurrentLevelName true))
  (bind _returnvalue_2 (SaveGame|CreateSaveGameObject "/Game/Blueprints/Save-Load/BP_SaveGame.BP_SaveGame_C"))
  (bind _output_get (Variables|Default|SetSaveData _returnvalue_2))
  (Variables|/Game/Blueprints/Save-Load/BP_SaveGame.BP_SaveGame_C|SetSavedLevel _output_get (Utilities|String|StringToName _returnvalue))
  ;[0.15 0.15 0.15 0.5] Gets Creature Data
  (bind _outactors (Actor|GetAllActorsOfClass "/Game/Blueprints/Creatures/BPP_Creature.BPP_Creature_C"))
  (for _array_element _outactors
    (bind _creaturesave (Default|SaveCreatureData _array_element))
    (Utilities|Array|Add (Variables|/Game/Blueprints/Save-Load/BP_SaveGame.BP_SaveGame_C|GetCreatures (Variables|Default|GetSaveData)) _creaturesave))
  ;[0.15 0.15 0.15 0.5] Stores latest creature ID for the spawner
  (bind _asgm_main_game_mode (Utilities|Casting|CastToGM_MainGameMode (Game|GetGameMode)))
  (Variables|/Game/Blueprints/Save-Load/BP_SaveGame.BP_SaveGame_C|SetLatestCreatureID (Variables|Default|GetSaveData) (Variables|/Game/Blueprints/GM_MainGameMode.GM_MainGameMode_C|GetLatestCreatureID _asgm_main_game_mode))
  (Utilities|FlowControl|Sequence
    (:then_0
      ;[0.15 0.15 0.15 0.5] Saves Cam Settings
      (bind _asbp_free_cam (Utilities|Casting|CastToBP_FreeCam (Game|Player|GetPlayerPawn 0)))
      (Variables|/Game/Blueprints/Save-Load/BP_SaveGame.BP_SaveGame_C|SetCamPos (Variables|Default|GetSaveData) (Transformation|GetWorldLocation (Variables|/Game/Blueprints/BP_FreeCam.BP_FreeCam_C|GetSphere _asbp_free_cam)))
      (Variables|/Game/Blueprints/Save-Load/BP_SaveGame.BP_SaveGame_C|SetCamPivot (Variables|Default|GetSaveData) (Variables|/Script/Engine.SceneComponent|GetRelativeRotation (Variables|/Game/Blueprints/BP_FreeCam.BP_FreeCam_C|GetPivot _asbp_free_cam)))
      (Variables|/Game/Blueprints/Save-Load/BP_SaveGame.BP_SaveGame_C|SetCamRot (Variables|Default|GetSaveData) (Variables|/Script/Engine.SceneComponent|GetRelativeRotation (Variables|/Game/Blueprints/BP_FreeCam.BP_FreeCam_C|GetSpringArm _asbp_free_cam)))
      (Variables|/Game/Blueprints/Save-Load/BP_SaveGame.BP_SaveGame_C|SetCamZoom (Variables|Default|GetSaveData) (Variables|/Script/Engine.SpringArmComponent|GetTargetArmLength (Variables|/Game/Blueprints/BP_FreeCam.BP_FreeCam_C|GetSpringArm _asbp_free_cam)))
      (Variables|/Game/Blueprints/Save-Load/BP_SaveGame.BP_SaveGame_C|SetHasCamSettings (Variables|Default|GetSaveData) true))
    (:then_1
      (Class|BPISaveGame|SaveGameData(Message) self))))

(fn LoadSavedData
  (bind _savedata (Variables|Default|GetSaveData))
  (for _array_element (Variables|/Game/Blueprints/Save-Load/BP_SaveGame.BP_SaveGame_C|GetCreatures (Variables|Default|GetSaveData))
    ;[0.15 0.15 0.15 0.5] Loads creatue data based on the struct
    (bind _returnvalue (Game|SpawnActorfromClass :Class (.CreatureClass (Utilities|Struct|BreakST_SavedCreatures _array_element)) :SpawnTransform (.Transform (Utilities|Struct|BreakST_SavedCreatures _array_element)) :CollisionHandlingOverride "AlwaysSpawn" :TransformScaleMethod "MultiplyWithRoot" :Held%20Traits (.HeldTraits (Utilities|Struct|BreakST_SavedCreatures _array_element)) :Instigator 0))
    (Default|LoadCreatureData _returnvalue _array_element)
    (Default|InitiateAppearance _returnvalue)
    (Default|LoadLabel _returnvalue))
  ;[0.15 0.15 0.15 0.5] Loads Cam settings
  (if (Variables|/Game/Blueprints/Save-Load/BP_SaveGame.BP_SaveGame_C|GetHasCamSettings _savedata)
    (bind _asbp_free_cam (Utilities|Casting|CastToBP_FreeCam (Game|Player|GetPlayerPawn 0)))
    (Transformation|SetWorldLocation (Variables|/Game/Blueprints/BP_FreeCam.BP_FreeCam_C|GetSphere _asbp_free_cam) (Variables|/Game/Blueprints/Save-Load/BP_SaveGame.BP_SaveGame_C|GetCamPos _savedata) false false)
    (Transformation|SetRelativeRotation (Variables|/Game/Blueprints/BP_FreeCam.BP_FreeCam_C|GetPivot _asbp_free_cam) (Variables|/Game/Blueprints/Save-Load/BP_SaveGame.BP_SaveGame_C|GetCamPivot _savedata) false false)
    (Transformation|SetRelativeRotation (Variables|/Game/Blueprints/BP_FreeCam.BP_FreeCam_C|GetSpringArm _asbp_free_cam) (Variables|/Game/Blueprints/Save-Load/BP_SaveGame.BP_SaveGame_C|GetCamRot _savedata) false false)
    (Variables|/Script/Engine.SpringArmComponent|SetTargetArmLength (Variables|/Game/Blueprints/BP_FreeCam.BP_FreeCam_C|GetSpringArm _asbp_free_cam) (Variables|/Game/Blueprints/Save-Load/BP_SaveGame.BP_SaveGame_C|GetCamZoom _savedata))))