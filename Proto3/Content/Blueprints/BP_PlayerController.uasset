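; Player controller that handles camera viewing, switching between a possessed free cam and a spectated creature.
; Holding the orbit input hides the cursor, switches to game-only input and forwards look input to the spectated creature's orbit camera.
; Mouse wheel steps spring-arm length within limits on the spectated creature, or on the free cam when none is valid.
; F blends the view to the free cam; the spectated creature is not assigned here.
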(event Input|EnhancedActionEvents|EnhancedInputActionIA_Look
  (params (ActionValue :type Vector%202D%20Structure) (ElapsedSeconds :type Float%20%28double-precision%29) (TriggeredSeconds :type Float%20%28double-precision%29) (InputAction :type Input%20Action%20Object%20Reference :default "/Game/Input/IA_Look.IA_Look"))
  (bind _spectatecreature (Variables|Default|GetSpectateCreature))
  ;[0.15 0.15 0.15 0.5] Enables input action for creature camera.
  (if (Variables|Default|GetisOrbit)
    (Utilities|IsValid _spectatecreature
      (:Is%20Valid
        (Default|OrbitCamera _spectatecreature (.x ActionValue) (.y ActionValue))))))

(event Input|EnhancedActionEvents|EnhancedInputActionIA_Orbit
  (params (ActionValue :type Boolean) (ElapsedSeconds :type Float%20%28double-precision%29) (TriggeredSeconds :type Float%20%28double-precision%29) (InputAction :type Input%20Action%20Object%20Reference :default "/Game/Input/IA_Orbit.IA_Orbit"))
  (bind _returnvalue (Game|GetPlayerController 0))
  ;[0.15 0.15 0.15 0.5] Sets ability to rotate camera around pivot point.
  (:Started
    (Variables|Default|SetisOrbit true)
    (Variables|/Script/Engine.PlayerController|SetbShowMouseCursor _returnvalue false)
    (Input|SetInputModeGameOnly _returnvalue false))
  (:Completed
    (Variables|Default|SetisOrbit false)
    (Variables|/Script/Engine.PlayerController|SetbShowMouseCursor _returnvalue true)
    (Input|SetInputModeGameandUI _returnvalue 0 "DoNotLock" true false)))

(event EventBeginPlay
  ;[0.15 0.15 0.15 0.5] Sets FreeCamRef
  (bind _asbp_free_cam (Utilities|Casting|CastToBP_FreeCam (Pawn|GetControlledPawn)))
  (Variables|Default|SetFreeCamRef _asbp_free_cam))

(event Input|MouseEvents|MouseWheelDown
  (params (Key :type Key%20Structure :default "None"))
  (bind _spectatecreature (Variables|Default|GetSpectateCreature))
  ;[0.6198 0.1504 0.5276 0.5] Zoom out
  (:Pressed
    (Utilities|IsValid _spectatecreature
      (:Is%20Valid
        (Variables|/Script/Engine.SpringArmComponent|SetTargetArmLength (Variables|/Game/Blueprints/Creatures/BPP_Creature.BPP_Creature_C|GetSpringArm (Variables|Default|GetSpectateCreature)) (Math|Float|Clamp(Float) (+ (Variables|/Script/Engine.SpringArmComponent|GetTargetArmLength (Variables|/Game/Blueprints/Creatures/BPP_Creature.BPP_Creature_C|GetSpringArm _spectatecreature)) 1e+02) 0.0 (Variables|Default|GetMaxArmLength))))
      (:Is%20Not%20Valid
        (Variables|/Script/Engine.SpringArmComponent|SetTargetArmLength (Variables|/Game/Blueprints/BP_FreeCam.BP_FreeCam_C|GetSpringArm (Variables|Default|GetFreeCamRef)) (Math|Float|Clamp(Float) (+ (Variables|/Script/Engine.SpringArmComponent|GetTargetArmLength (Variables|/Game/Blueprints/BP_FreeCam.BP_FreeCam_C|GetSpringArm (Variables|Default|GetFreeCamRef))) 1e+02) 0.0 (Variables|Default|GetMaxArmLength)))))))

(event Input|MouseEvents|MouseWheelUp
  (params (Key :type Key%20Structure :default "None"))
  ;[0.6198 0.1504 0.5276 0.5] Zoom in
  (:Pressed
    (Utilities|IsValid (Variables|Default|GetSpectateCreature)
      (:Is%20Valid
        (if (>= (- (Variables|/Script/Engine.SpringArmComponent|GetTargetArmLength (Variables|/Game/Blueprints/Creatures/BPP_Creature.BPP_Creature_C|GetSpringArm (Variables|Default|GetSpectateCreature))) 1e+02) (Variables|Default|GetMinArmLength))
          (Variables|/Script/Engine.SpringArmComponent|SetTargetArmLength (Variables|/Game/Blueprints/Creatures/BPP_Creature.BPP_Creature_C|GetSpringArm (Variables|Default|GetSpectateCreature)) (- (Variables|/Script/Engine.SpringArmComponent|GetTargetArmLength (Variables|/Game/Blueprints/Creatures/BPP_Creature.BPP_Creature_C|GetSpringArm (Variables|Default|GetSpectateCreature))) 1e+02))))
      (:Is%20Not%20Valid
        (if (>= (- (Variables|/Script/Engine.SpringArmComponent|GetTargetArmLength (Variables|/Game/Blueprints/BP_FreeCam.BP_FreeCam_C|GetSpringArm (Variables|Default|GetFreeCamRef))) 1e+02) (Variables|Default|GetMinArmLength))
          (Variables|/Script/Engine.SpringArmComponent|SetTargetArmLength (Variables|/Game/Blueprints/BP_FreeCam.BP_FreeCam_C|GetSpringArm (Variables|Default|GetFreeCamRef)) (- (Variables|/Script/Engine.SpringArmComponent|GetTargetArmLength (Variables|/Game/Blueprints/BP_FreeCam.BP_FreeCam_C|GetSpringArm (Variables|Default|GetFreeCamRef))) 1e+02)))))))

(event Input|KeyboardEvents|F
  (params (Key :type Key%20Structure :default "None"))
  (bind _freecamref (Variables|Default|GetFreeCamRef))
  ;[0.15 0.15 0.15 0.5] Sets camera to FreeCam.
  (:Pressed
    (Utilities|IsValid _freecamref
      (:Is%20Valid
        (Game|Player|SetViewTargetwithBlend (Game|GetPlayerController 0) _freecamref 0.5 "VTBlend_Linear" 0.0 false)))))

(fn ConstructionScript)